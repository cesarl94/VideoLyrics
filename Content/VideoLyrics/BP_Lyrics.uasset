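; BP_Lyrics is a video-lyrics actor that shows timed verse textures on a static mesh for one song or a playlist.
; Tick finds the current song from real time, loads numbered verse textures synchronously and alternates two material slots, fading each with its own timeline.
; It also drives a black-curtain fade at both ends of the total duration.
; BeginPlay validates setup and applies a no-tonemapping post-process material that adjusts for the render-pipeline game mode.
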(event Custom|AnimateLyric
  (params (LyricId :type Integer) (Open :type Boolean) (RowId :type Integer) (SongId :type Integer))
  (bind _returnvalue (Utilities|Select :Index LyricId :Option%200 "A" :Option%201 "B"))
  (bind _timelinesdata (Variables|Default|GettimelinesData))
  (bind _dynamicmaterialinstance (Variables|Default|GetDynamicMaterialInstance))
  (bind _output (Utilities|Array|Get(acopy) _timelinesdata LyricId))
  (bind (_opened _timeline) (Utilities|Struct|BreakFTimelineData _output))
  (if Open
    (if _opened
      (Development|PrintString (Utilities|String|Append "Error trying to " (select Open "open " "close ") _returnvalue " when it is already closed" (select Open "opened." "closed.")) true true "(R=1.000000,G=0.000000,B=0.000000,A=1.000000)" :!label _label)
      (else
        (bind (_verse _sucess) (CallFunction|GetVerse SongId RowId))
        (if _sucess
          (Utilities|Struct|SetmembersinFTimelineData _output true RowId 1.0)
          (Rendering|Material|SetScalarParameterValue _dynamicmaterialinstance "ShowAFactor" (- 1.0 (Math|Conversions|ToFloat(Integer) LyricId)) :!class /Script/Engine.MaterialInstanceDynamic)
          (Rendering|Material|SetTextureParameterValue _dynamicmaterialinstance (Utilities|String|StringToName (Utilities|String|Append "Lyric" _returnvalue)) (Utilities|Struct|BreakFVerse _verse))
          (Components|Timeline|SetPlayRate _timeline (/ 1.0 (Utilities|Struct|BreakFSongData (Utilities|Array|Get(acopy) (Variables|DefaultValues|GetSongData) SongId))))
          (bind _returnvalue_2 (Rendering|Material|GetScalarParameterValue _dynamicmaterialinstance (Utilities|String|StringToName (Utilities|String|Append "Alpha" _returnvalue)) :!class /Script/Engine.MaterialInstanceDynamic :!label _label_2))
          (Utilities|Struct|SetmembersinFTimelineData _output _returnvalue_2)
          (Components|Timeline|PlayfromStart _timeline))))
    (elif _opened
      (Utilities|Struct|SetmembersinFTimelineData _output false 0.0)
      (goto _label_2)
      (else
        (goto _label)))))

(event EventBeginPlay
  (if (Utilities|IsValidClass (Variables|DefaultValues|GetRenderPipelineGameMode))
    (Utilities|IsValid (Variables|DefaultValues|GetMaterial)
      (:Is%20Valid
        (if (> (Utilities|Array|Length (Variables|DefaultValues|GetSelectedSongs)) 0)
          (bind _returnvalue (Actor|GetActorOfClass "/Script/Engine.PostProcessVolume"))
          (Utilities|IsValid _returnvalue
            (:Is%20Valid
              (bind _returnvalue_2 (Rendering|Material|CreateDynamicMaterialInstance "/Game/Materials/M_NoToneMapping.M_NoToneMapping" "None" "None" :!class /Script/Engine.KismetMaterialLibrary))
              (bind _structout (Utilities|Struct|SetmembersinWeightedBlendables (|Copy (Utilities|Struct|BreakPostProcessSettings (Variables|/Script/Engine.PostProcessVolume|GetSettings _returnvalue))) (Utilities|Array|MakeArray (Utilities|Struct|MakeWeightedBlendable 1.0 _returnvalue_2))))
              (bind _structout_2 (Utilities|Struct|SetmembersinPostProcessSettings (|Copy (Variables|/Script/Engine.PostProcessVolume|GetSettings _returnvalue)) _structout))
              (Variables|/Script/Engine.PostProcessVolume|SetSettings _returnvalue _structout_2)
              (bind _returnvalue_3 (Actor|GetActorOfClass (Variables|DefaultValues|GetRenderPipelineGameMode)))
              (Rendering|Material|SetScalarParameterValue _returnvalue_2 "IncidenceFactor" (- 1.0 (Math|Conversions|ToFloat(Boolean) (Utilities|IsValid _returnvalue_3))) :!class /Script/Engine.MaterialInstanceDynamic)
              (bind _returnvalue_4 (Rendering|Material|CreateDynamicMaterialInstance (Variables|Debug|GetStaticMeshComponent) 0 (Variables|DefaultValues|GetMaterial) "None" :!class /Script/Engine.PrimitiveComponent))
              (Variables|Default|SetDynamicMaterialInstance _returnvalue_4)
              (for _index (range 0 1)
                (Utilities|Array|SetArrayElem (Variables|Default|GetTimelinesData) _index (Utilities|Struct|MakeFTimelineData (Utilities|Array|Get(acopy) (Utilities|Array|MakeArray 0 -1) _index) (Utilities|Array|Get(acopy) (Utilities|Array|MakeArray (Variables|Default|GetTimelineA) (Variables|Default|GetTimelineB)) _index)) true)))
            (:Is%20Not%20Valid
              (Development|PrintString "You need a PostProcessVolume in the level" true true "(R=1.000000,G=0.000000,B=0.000000,A=1.000000)" 5.0)
              (Actor|Tick|SetActorTickEnabled false)))
          (else
            (Development|PrintString "You need to specify song Id's in the BP_Lyrics. You need at least one" true true "(R=1.000000,G=0.000000,B=0.000000,A=1.000000)" 5.0)
            (Actor|Tick|SetActorTickEnabled false))))
      (:Is%20Not%20Valid
        (Development|PrintString "You need to specify a Material in the BP_Lyrics" true true "(R=1.000000,G=0.000000,B=0.000000,A=1.000000)" 5.0)
        (Actor|Tick|SetActorTickEnabled false)))
    (else
      (Development|PrintString "You need to specify the Game Mode used in the Render Pipeline (Setted in \"Game Overrides\" section in Movie Render Settings) in the BP_Lyrics object also" true true "(R=1.000000,G=0.000000,B=0.000000,A=1.000000)" 5.0)
      (Actor|Tick|SetActorTickEnabled false))))

(event EventTick
  (params (DeltaSeconds :type Float%20%28single-precision%29))
  (bind _returnvalue (CallFunction|GetTotalDuration))
  (bind _returnvalue_2 (/ _returnvalue 2.0))
  (Variables|Default|SetrealTimeSeconds (Utilities|Time|GetRealTimeSeconds))
  (Utilities|FlowControl|Sequence
    (:then_0
      (if (!= (Utilities|Array|Length (Variables|DefaultValues|GetSelectedSongs)) 1)
        (Utilities|FlowControl|Sequence)))
    (:then_1
      (Rendering|Material|SetScalarParameterValue (Variables|Default|GetDynamicMaterialInstance) "BlackCurtainOpacity" (- 1.0 (Math|Float|Clamp(Float) (- _returnvalue_2 (Math|Float|Absolute(Float) (- (Variables|Default|GetRealTimeSeconds) _returnvalue_2))))) :!class /Script/Engine.MaterialInstanceDynamic)
      (bind (_songidonplaylist _songidworld _delta) (CallFunction|GetCurrentSongData))
      (if (!= _songidworld -1)
        (if (!= _songidonplaylist (Variables|Default|GetSongPlaylistId))
          (Variables|Default|SetSongPlaylistId _songidonplaylist)
          (Variables|Default|SetNextRow 0))
        (Utilities|FlowControl|Sequence
          (:then_0
            (for _index (range 0 1)
              (if (.Opened (Utilities|Struct|BreakFTimelineData (Utilities|Array|Get(acopy) (Variables|Default|GetTimelinesData) _index)))
                (bind _verse (CallFunction|GetVerse _songidworld (.Row (Utilities|Struct|BreakFTimelineData (Utilities|Array|Get(acopy) (Variables|Default|GetTimelinesData) _index)))))
                (if (>= _delta (- (Utilities|Struct|BreakFVerse _verse) (Utilities|Struct|BreakFSongData (Utilities|Array|Get(acopy) (Variables|DefaultValues|GetSongData) _songidworld))))
                  (CallFunction|AnimateLyric _index false (.Row (Utilities|Struct|BreakFTimelineData (Utilities|Array|Get(acopy) (Variables|Default|GetTimelinesData) _index))) _songidworld)))))
          (:then_1
            (bind (_verse_2 _sucess) (CallFunction|GetVerse _songidworld (Variables|Default|GetNextRow)))
            (if _sucess
              (if (>= _delta (Utilities|Struct|BreakFVerse _verse_2))
                (CallFunction|AnimateLyric (select (Variables|Default|GetNextIsA) 0 1) true (Variables|Default|GetNextRow) _songidworld)
                (Math|Integer|IncrementInt (Variables|Default|GetNextRow)
                  (:%20%20
                    (Variables|Default|SetNextIsA (not (Variables|Default|GetNextIsA)))))))))))))

(fn ConstructionScript
  (Rendering|Material|SetMaterial (Variables|Debug|GetStaticMeshComponent) 0 (Variables|DefaultValues|GetMaterial)))

(fn GetCurrentSongData
  (bind _selectedsongs (Variables|DefaultValues|GetSelectedSongs))
  (bind _selectedsongs_2 (Variables|DefaultValues|GetSelectedSongs))
  (bind _realtimeseconds (Variables|Default|GetRealTimeSeconds))
  (bind _returnvalue (Utilities|Array|Length _selectedsongs_2))
  (bind _returnvalue_2 (- _returnvalue 1))
  (bind _output (Utilities|Array|Get(acopy) _selectedsongs_2 _returnvalue_2))
  (if (== (Utilities|Array|Length _selectedsongs) 1)
    (return 0 (Utilities|Array|Get(acopy) _selectedsongs) (Variables|Default|GetRealTimeSeconds))
    (else
      (for (_array_element _array_index) (Variables|DefaultValues|GetSelectedSongs)
        (if (and (<= (.Begins (CallFunction|GetPlaylistSongTimes _array_index)) _realtimeseconds) (> (.Ends (CallFunction|GetPlaylistSongTimes _array_index)) _realtimeseconds))
          (return _array_index _array_element (- _realtimeseconds (.Begins (CallFunction|GetPlaylistSongTimes _array_index))))))
      (return _returnvalue_2 _output (- (Variables|Default|GetRealTimeSeconds) (.Begins (CallFunction|GetPlaylistSongTimes _output)))))))

(fn GetPlaylistSongTimes
  (params (PlaylistSongId :type Integer))
  (return (Utilities|Select :Index PlaylistSongId :Option%200 0.0 :Option%201 0.0 :Option%202 0.0 :Option%203 0.0 :Option%204 0.0) (Utilities|Select :Index PlaylistSongId :Option%200 0.0 :Option%201 0.0 :Option%202 0.0 :Option%203 0.0 :Option%204 0.0)))

(fn GetVerse
  (params (SongId :type Integer) (RowId :type Integer))
  (bind _songdata (Variables|DefaultValues|GetSongData))
  (bind _output (Utilities|Array|Get(acopy) _songdata SongId))
  (bind (_initseconds _endseconds _filenamewithallzeros _filenamedigits _firstframeid) (Utilities|Struct|BreakFSongData _output))
  (if (or (< RowId 0) (>= RowId (Utilities|Array|Length _initseconds)))
    (return "" false)
    (else
      (bind _returnvalue (Utilities|LoadAssetBlocking (Class|KismetSystemLibrary|ToSoftObjRef(SoftObjPath) (Utilities|MakeSoftObjectPath (Utilities|String|Replace _filenamewithallzeros (Utilities|InttoString 0 _filenamedigits) (Utilities|InttoString (+ _firstframeid RowId) _filenamedigits) "CaseSensitive")))))
      (return (Utilities|Struct|MakeFVerse (.AsTexture%202D (Utilities|Casting|CastToTexture2D _returnvalue)) (Utilities|Array|Get(acopy) _initseconds (LocalVariables|GetrowId)) (Utilities|Array|Get(acopy) _endseconds (LocalVariables|GetrowId))) true))))

(fn InttoString
  (params (Integer :type Integer) (DigitsCount :type Integer))
  (bind _output_get (LocalVariables|SetTempString (Utilities|String|ToString(Integer) Integer)))
  (for _index (range (Utilities|String|Len _output_get) (- DigitsCount 1))
    (LocalVariables|SetTempString (Utilities|String|Append "0" (LocalVariables|GetTempString))))
  (return (LocalVariables|GetTempString)))

(fn Linearstep
  (params (InputData0 :type Float%20%28double-precision%29) (InputData1 :type Float%20%28double-precision%29) (Input :type Float%20%28double-precision%29) (Clamp :type Boolean))
  (bind _returnvalue (- InputData1 InputData0))
  (bind _returnvalue_2 (- Input InputData0))
  (bind _returnvalue_3 (/ _returnvalue_2 _returnvalue))
  (if (== _returnvalue 0.0)
    (return 1.0)
    (else
      (return (select Clamp (Math|Float|Clamp(Float) _returnvalue_3) _returnvalue_3)))))

(fn RuleOfFive
  (params (InputDataA :type Float%20%28double-precision%29) (OutputDataA :type Float%20%28double-precision%29) (InputDataB :type Float%20%28double-precision%29) (OutputDataB :type Float%20%28double-precision%29) (Input :type Float%20%28double-precision%29) (Clamp :type Boolean))
  (bind _returnvalue (Utilities|Linearstep InputDataA InputDataB Input Clamp)) ; t
  (return (+ OutputDataA (* (- OutputDataB OutputDataA) _returnvalue))))

(fn GetTotalDuration
  (for _array_element (Variables|DefaultValues|GetSelectedSongs)
    (LocalVariables|SetCurrentDuration (+ (LocalVariables|GetCurrentDuration) (.SongDuration (Utilities|Struct|BreakFSongData (Utilities|Array|Get(acopy) (Variables|DefaultValues|GetSongData) _array_element))))))
  (return (LocalVariables|GetCurrentDuration)))